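; BP_BasketStatic is a basket target for a ball minigame that removes itself on timeout or when hit.
; Tick counts Lifetime down by world delta seconds and destroys the actor once it reaches zero.
; A BoxCollision overlap with a BP_BallMinigame prints "SumarPuntaje" (add score) and destroys the basket, without changing any score here.
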(event OnComponentBeginOverlap(Grid(BoxCollision))
  (params (OverlappedComponent :type Primitive%20Component%20Object%20Reference) (OtherActor :type Actor%20Object%20Reference) (OtherComp :type Primitive%20Component%20Object%20Reference) (OtherBodyIndex :type Integer) (bFromSweep :type Boolean) (SweepResult :type Hit%20Result%20Structure%20%28by%20ref%29))
  (Utilities|Casting|CastToBP_BallMinigame OtherActor)
  (Development|PrintString "SumarPuntaje")
  (Actor|DestroyActor))

(event EventTick
  (params (DeltaSeconds :type Float%20%28single-precision%29))
  (if (<= (Variables|Default|GetLifetime) 0.0)
    (Actor|DestroyActor)
    (else
      (Variables|Default|SetLifetime (- (Variables|Default|GetLifetime) (Utilities|Time|GetWorldDeltaSeconds))))))

(fn ConstructionScript)
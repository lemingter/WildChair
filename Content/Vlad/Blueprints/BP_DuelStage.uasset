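; BP_DuelStage is the stage for a VR ball-and-basket minigame, active while a VRPawn overlaps its detection box.
; Entering spawns a ball, and Tick runs countdowns that periodically spawn more balls and baskets while the player stays inside.
; Each basket takes one of twelve random positions and receives a reference to the stage.
; Two separate random rolls pick static, horizontal or vertical baskets, so the odds favor vertical.
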(event OnComponentBeginOverlap(PlayerDetector(BoxCollision))
  (params (OverlappedComponent :type Primitive%20Component%20Object%20Reference) (OtherActor :type Actor%20Object%20Reference) (OtherComp :type Primitive%20Component%20Object%20Reference) (OtherBodyIndex :type Integer) (bFromSweep :type Boolean) (SweepResult :type Hit%20Result%20Structure%20%28by%20ref%29))
  ;[0.3 0.81 0.7 0.12] Deteccion Del Personaje
  (Utilities|Casting|CastToVRPawn OtherActor)
  (Variables|Default|SetPlayerIn true)
  (CallFunction|GenerateBall))

(event OnComponentEndOverlap(PlayerDetector(BoxCollision))
  (params (OverlappedComponent :type Primitive%20Component%20Object%20Reference) (OtherActor :type Actor%20Object%20Reference) (OtherComp :type Primitive%20Component%20Object%20Reference) (OtherBodyIndex :type Integer))
  ;[0.3 0.81 0.7 0.12] Deteccion Del Personaje
  (Utilities|Casting|CastToVRPawn OtherActor)
  (Variables|Default|SetPlayerIn false))

(event Custom|GenerateBall
  ;[0.41 0.29 0.55 0.79] Funcion Para Spawnear Un Pelota
  (Game|SpawnActorfromClass "/Game/Vlad/Blueprints/BP_BallMinigame.BP_BallMinigame_C" (Transformation|GetWorldTransform (Variables|Default|GetBallSpaawn)) "Undefined" "MultiplyWithRoot" 0 0))

(event Custom|SpawnBallCounter
  ;[0.2 0.42 0.13] Funcion Para Determinar Si Se Puede Spawnear Una Pelota
  (if (<= (Variables|Default|GetSpawnBallTimer) 0.0)
    (CallFunction|GenerateBall)
    (Variables|Default|SetSpawnBallTimer 1e+01)
    (else
      (Variables|Default|SetSpawnBallTimer (- (Variables|Default|GetSpawnBallTimer) (Utilities|Time|GetWorldDeltaSeconds))))))

(event Custom|SelectBasketSpawn
  ;[0.98 0.25 0.7 0.63] Seleccionar Una Posicion Para Spawnear La Canasta
  (switch int (Math|Random|RandomInteger 12)
    (:0
      (CallFunction|SelectBasketType (Transformation|GetWorldTransform (Variables|Default|GetBasketPosition1))))
    (:1
      (CallFunction|SelectBasketType (Transformation|GetWorldTransform (Variables|Default|GetBasketPosition2))))
    (:2
      (CallFunction|SelectBasketType (Transformation|GetWorldTransform (Variables|Default|GetBasketPosition3))))
    (:3
      (CallFunction|SelectBasketType (Transformation|GetWorldTransform (Variables|Default|GetBasketPosition4))))
    (:4
      (CallFunction|SelectBasketType (Transformation|GetWorldTransform (Variables|Default|GetBasketPosition5))))
    (:5
      (CallFunction|SelectBasketType (Transformation|GetWorldTransform (Variables|Default|GetBasketPosition6))))
    (:6
      (CallFunction|SelectBasketType (Transformation|GetWorldTransform (Variables|Default|GetBasketPosition7))))
    (:7
      (CallFunction|SelectBasketType (Transformation|GetWorldTransform (Variables|Default|GetBasketPosition8))))
    (:8
      (CallFunction|SelectBasketType (Transformation|GetWorldTransform (Variables|Default|GetBasketPosition9))))
    (:9
      (CallFunction|SelectBasketType (Transformation|GetWorldTransform (Variables|Default|GetBasketPosition10))))
    (:10
      (CallFunction|SelectBasketType (Transformation|GetWorldTransform (Variables|Default|GetBasketPosition11))))
    (:11
      (CallFunction|SelectBasketType (Transformation|GetWorldTransform (Variables|Default|GetBasketPosition12))))))

(event Custom|SelectBasketType
  (params (BasketPosition :type Transform))
  (bind _returnvalue (Math|Random|RandomInteger 3))
  ;[0.53 0.39 0.94 0.45] Spawnear Una Canasta Aleatoria
  (if (== _returnvalue 0)
    (bind _returnvalue_2 (Game|SpawnActorfromClass "/Game/Vlad/Blueprints/BP_BasketStatic.BP_BasketStatic_C" BasketPosition "Undefined" "MultiplyWithRoot" 0 0))
    (Variables|/Game/Vlad/Blueprints/BP_BasketStatic.BP_BasketStatic_C|SetDuelStage_Reference _returnvalue_2 self)
    (elif (== _returnvalue 1)
      (bind _returnvalue_3 (Game|SpawnActorfromClass "/Game/Vlad/Blueprints/BP_BasketHorizontal.BP_BasketHorizontal_C" BasketPosition "Undefined" "MultiplyWithRoot" 0 0))
      (Variables|/Game/Vlad/Blueprints/BP_BasketHorizontal.BP_BasketHorizontal_C|SetDuelStage_Reference _returnvalue_3 self)
      (else
        (bind _returnvalue_4 (Game|SpawnActorfromClass "/Game/Vlad/Blueprints/BP_BasketVertical.BP_BasketVertical_C" BasketPosition "Undefined" "MultiplyWithRoot" 0 0))
        (Variables|/Game/Vlad/Blueprints/BP_BasketVertical.BP_BasketVertical_C|SetDuelStage_Reference _returnvalue_4 self)))))

(event Custom|SpawnBasketCounter
  ;[0 0.85 0.3 0.02] Contador Para Spawnear Una Nueva Canasta
  (if (<= (Variables|Default|GetSpawnBasketTimer) 0.0)
    (CallFunction|SelectBasketSpawn)
    (Variables|Default|SetSpawnBasketTimer 15.0)
    (else
      (Variables|Default|SetSpawnBasketTimer (- (Variables|Default|GetSpawnBasketTimer) (Utilities|Time|GetWorldDeltaSeconds))))))

(event EventTick
  (params (DeltaSeconds :type Float%20%28single-precision%29))
  (if (Variables|Default|GetPlayerIn)
    (CallFunction|SpawnBallCounter)
    (CallFunction|SpawnBasketCounter)))

(fn ConstructionScript)
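; BP_BallMinigame is a grabbable minigame ball that destroys itself when its lifetime runs out.
; Each tick it counts LifeTime down while GrabComponent reports it is not held, destroying the actor at zero.
; While held the countdown pauses and RestartLifetime is called, but its DoOnce has no reset, so the timer refills only on the first call.
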(event Custom|Restart%20Lifetime
  ;[0.96 0.45 0.8 0.16] Resetear El Lifetime
  (Utilities|FlowControl|DoOnce false
    (:Completed
      (Variables|Default|SetLifeTime 3e+01))))

(event EventTick
  (params (DeltaSeconds :type Float%20%28single-precision%29))
  (if (Variables|/Game/VRTemplate/Blueprints/GrabComponent.GrabComponent_C|GetbIsHeld (Variables|Default|GetGrabComponent))
    (CallFunction|RestartLifetime)
    (elif (<= (Variables|Default|GetLifeTime) 0.0)
      (Actor|DestroyActor)
      (else
        (Variables|Default|SetLifeTime (- (Variables|Default|GetLifeTime) (Utilities|Time|GetWorldDeltaSeconds)))))))

(fn ConstructionScript)
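; BP_BasketVertical is a short-lived basket target that awards points in a duel stage ball minigame.
; Tick counts Lifetime down by world delta time and destroys the actor once it runs out.
; When a BP_BallMinigame overlaps its box collision, it adds PointsToAdd to the BasketScore of the referenced BP_DuelStage, then destroys itself.
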(event OnComponentBeginOverlap(Grid(BoxCollision))
  (params (OverlappedComponent :type Primitive%20Component%20Object%20Reference) (OtherActor :type Actor%20Object%20Reference) (OtherComp :type Primitive%20Component%20Object%20Reference) (OtherBodyIndex :type Integer) (bFromSweep :type Boolean) (SweepResult :type Hit%20Result%20Structure%20%28by%20ref%29))
  (Utilities|Casting|CastToBP_BallMinigame OtherActor)
  (CallFunction|AddPoints)
  (Actor|DestroyActor))

(event Custom|AddPoints
  ;[0.69 0.49 0.27 0.58] Añadir puntos al DuelStage
  (bind _asbp_duel_stage (Utilities|Casting|CastToBP_DuelStage (Variables|Default|GetDuelStage_Reference)))
  (Variables|/Game/Vlad/Blueprints/BP_DuelStage.BP_DuelStage_C|SetBasketScore _asbp_duel_stage (+ (Variables|/Game/Vlad/Blueprints/BP_DuelStage.BP_DuelStage_C|GetBasketScore _asbp_duel_stage) (Variables|Default|GetPointsToAdd))))

(event EventTick
  (params (DeltaSeconds :type Float%20%28single-precision%29))
  (if (<= (Variables|Default|GetLifetime) 0.0)
    (Actor|DestroyActor)
    (else
      (Variables|Default|SetLifetime (- (Variables|Default|GetLifetime) (Utilities|Time|GetWorldDeltaSeconds))))))

(fn ConstructionScript)
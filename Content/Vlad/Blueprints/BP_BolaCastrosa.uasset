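; BP_BolaCastrosa is a grabbable VR collectible that adds to the player's score when picked up.
; Its GrabComponent's OnGrabbed event waits two seconds, then calls AddToInventory, which increments Score on the VRPawn found by class lookup and prints it.
; It then spawns an explosion particle and collect sound at its location and destroys itself.
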(event OnGrabbed(GrabComponent)
  (params (Motion%20controller :type Motion%20Controller%20Component%20Object%20Reference))
  (bind _returnvalue (Transformation|GetActorLocation))
  (Utilities|FlowControl|Delay 2.0)
  (CallFunction|AddtoInventory)
  (Effects|SpawnEmitteratLocation "/Game/StarterContent/Particles/P_Explosion.P_Explosion" _returnvalue)
  (Audio|PlaySoundatLocation "/Game/Vlad/Audio/Item_Collect_SFX.Item_Collect_SFX" _returnvalue "0, 0, 0" 1.0 1.0 0.0 0 0 0 0)
  (Actor|DestroyActor))

(event Custom|AddToInventory
  ;[0.09 0.75 0.12 0.98] Incluir el coleccionable al inventario
  (bind _returnvalue (Actor|GetActorOfClass "/Game/VRTemplate/Blueprints/VRPawn.VRPawn_C"))
  (bind _result (Math|Integer|IncrementInt (Variables|/Game/VRTemplate/Blueprints/VRPawn.VRPawn_C|GetScore _returnvalue))
    (:%20%20
      (bind _output_get (Variables|/Game/VRTemplate/Blueprints/VRPawn.VRPawn_C|SetScore _returnvalue _result))
      (Development|PrintString (Utilities|String|ToString(Integer) _output_get)))))

(fn ConstructionScript)